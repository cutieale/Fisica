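; BP_PracticeTarget is a destructible target that shatters when it takes any damage.
; On damage it hides and disables collision on the static mesh, reveals the physics-simulated Geometry Collection, and breaks it with a radial impulse that applies strain.
; The first Chaos removal event turns off removal notifications and destroys the actor after a short delay.
; The Geometry Collection is made unwalkable at BeginPlay.
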(event `self.ReceiveBeginPlay`
  (`PrimitiveComponent.SetWalkableSlopeOverride` (`self.GeometryCollection`) (make `WalkableSlopeOverride` "WalkableSlope_Unwalkable")))

(event `self.ReceiveAnyDamage`
  (params (Damage :type "Float (single-precision)") (DamageType :type "DamageType Object Reference") (InstigatedBy :type "Controller Object Reference") (DamageCauser :type "Actor Object Reference"))
  (bind _geometrycollection (`self.GeometryCollection`))
  (bind _staticmesh (`self.StaticMesh`))
  (`SceneComponent.SetHiddenInGame` _staticmesh true false)
  (`PrimitiveComponent.SetCollisionEnabled` _staticmesh "NoCollision")
  (`SceneComponent.SetHiddenInGame` _geometrycollection false false)
  (`PrimitiveComponent.SetSimulatePhysics` _geometrycollection true)
  (`PhysicsObjectBlueprintLibrary.ApplyRadialImpulse` (`self.GeometryCollection`) (`SceneComponent.K2_GetComponentLocation` (`self.GeometryCollection`)) 100.0 50000.0 "RIF_Constant" true 5000000.0))

(event `self.GeometryCollection.OnChaosRemovalEvent`
  (params (RemovalEvent :type "ChaosRemovalEvent Structure (by ref)"))
  (`GeometryCollectionComponent.SetNotifyRemovals` (`self.GeometryCollection`) false)
  (`KismetSystemLibrary.Delay` 1.0)
  (`self.K2_DestroyActor`))

(fn `UserConstructionScript`)